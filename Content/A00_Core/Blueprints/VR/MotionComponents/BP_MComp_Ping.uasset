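; BP_MComp_Ping is a VR motion component that lets a player place a ping in the world.
; When the Ping function input is set, it runs a short visibility line trace forward from SelectSearchArrow.
; The hit location, or the trace end on a miss, goes to the VR pawn's SpawnPing, colored by the player state's index color.
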(event EventFunctionInput
  (params (Function :type Name :default "None") (Set :type Boolean))
  ;[1 1 1] KeyInputs
  (|CallParentFunction Function Set)
  (switch name Function
    (:Ping
      ;[1 1 1] Ping
      (if Set
        (bind _impactpoint (|TraceForPing))
        (Default|SpawnPing (Variables|Default|GetVRPawn) _impactpoint 2.0 8.0 (Default|GetIndexColor (Default|GetPlayerState (Variables|Default|GetVRPawn))))))))

(fn ConstructionScript)