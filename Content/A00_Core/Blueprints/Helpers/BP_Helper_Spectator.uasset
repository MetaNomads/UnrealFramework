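; BP_Helper_Spectator is a helper actor that carries a 2D scene capture component, apparently to provide a spectator view.
; Its construction script copies the exposed post-process settings and field of view onto the capture component.
; At BeginPlay it binds to its MasterActor's OnDestroyed event to destroy itself along with that actor, or prints a message if no MasterActor is set.
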(event Custom|OnDestroyed_Event_1
  (params (DestroyedActor :type Actor%20Object%20Reference))
  ;[1 1 1] Auto Destroy
  (Actor|DestroyActor))

(event EventBeginPlay
  (bind _self self)
  ;[1 1 1] Auto Destroy
  (bind _masteractor (Variables|Helper|GetMasterActor)
    (:then
      (Game|AssignOnDestroyed _masteractor (delegate Custom|OnDestroyed_Event_1)))
    (:else
      (CallFunction|PrintMessage _self "NewEnumerator0" _self "Missing Master Actor" 1))))

(fn ConstructionScript
  (bind _scenecapturecomponent2d (Variables|Default|GetSceneCaptureComponent2D))
  (Variables|/Script/Engine.SceneCaptureComponent2D|SetPostProcessSettings _scenecapturecomponent2d (Variables|Default|GetPostProcessSettings))
  (Variables|/Script/Engine.SceneCaptureComponent2D|SetFOVAngle _scenecapturecomponent2d (Variables|Default|GetFOVAngle)))